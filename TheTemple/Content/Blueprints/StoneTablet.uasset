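; StoneTablet Blueprint that rotates stone tablet actors around their yaw axis.
; While Rotate is set, Tick continuously spins TargetObject in local space at RotateSpeed, scaled by frame time.
; Separately, RotateStoneTablet snaps a given tablet's yaw to a stored angle, then advances that angle by a fixed step, with a debug print.
; RotateAmountOfDegrees only records an actor's current yaw; other rotation experiments remain unconnected.
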(event `self.ReceiveBeginPlay`)

(event `self.ReceiveTick`
  (params (DeltaSeconds :type "Float (single-precision)"))
  (if (`self.Rotate`)
    (`Actor.K2_AddActorLocalRotation` (`self.TargetObject`) (* (`KismetMathLibrary.MakeRotator` 0.0 0.0 (`self.rotateSpeed`)) DeltaSeconds) false false)))

(fn `RotateAmountOfDegrees`
  (params (Actor :type "Actor Object Reference"))
  (set `self.ActorRotation` (.yaw (`Actor.K2_GetActorRotation` Actor))))

(fn `RotateStoneTablet`
  (params (Tablet :type "Actor Object Reference"))
  (locals (NewLocalVar_0 :type "Transform Structure"))
  (bind _degrees (`self.Degrees`))
  (`KismetSystemLibrary.PrintString` "Hello")
  (`Actor.K2_SetActorRotation` Tablet (`KismetMathLibrary.MakeRotator` (.roll (`Actor.K2_GetActorRotation` Tablet)) (.pitch (`Actor.K2_GetActorRotation` Tablet)) _degrees) false)
  (set `self.Degrees` (+ _degrees 15.0)))