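; OpeningDoor is a puzzle-check Blueprint that plays the ExitDoor level sequence once five rotation objects all report Complete.
; Tick polls the five Complete flags through nested branches, then calls SequencePlayer to create a level sequence player and play it.
; No guard stops the trigger, so a new player is created every tick while all five stay complete.
; The CheckingStonetabletRotation function is an empty stub.
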(event `self.ReceiveTick`
  (params (DeltaSeconds :type "Float (single-precision)"))
  (if (`/Game/Blueprints/CheckPuzzle/CheckFirstRingRotation.Complete` (`self.FirstRotation`))
    (if (`/Game/Blueprints/CheckPuzzle/CheckSecondRingRotation.Complete` (`self.SecondRotation`))
      (if (`/Game/Blueprints/CheckPuzzle/CheckThirdRingRotation.Complete` (`self.ThirdRotation`))
        (if (`/Game/Blueprints/CheckPuzzle/CheckFourRingRotation.Complete` (`self.FourRotation`))
          (if (`/Game/Blueprints/CheckPuzzle/CheckFifthRingRotation.Complete` (`self.FifthRotation`))
            (`self.SequencePlayer`)))))))

(event `SequencePlayer`
  (bind (_outactor _returnvalue) (`LevelSequencePlayer.CreateLevelSequencePlayer` (`self.ExitDoor`)))
  (`MovieSceneSequencePlayer.Play` _returnvalue))

(event `self.ReceiveBeginPlay`)

(fn `CheckingStonetabletRotation`)

(fn `UserConstructionScript`)