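; Puzzle checker for the fourth rotating ring, which tracks whether the ring sits at its target angle.
; On BeginPlay it registers itself as FourRotation on OpeningDoor, giving the door a reference to its state.
; Every Tick it wraps the actor's yaw with modulo 360 and sets Complete only while that value is within a narrow tolerance around 60 degrees.
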(event `self.ReceiveBeginPlay`
  (set `/Game/Blueprints/CheckPuzzle/OpeningDoor.FourRotation` self (`self.OpeningDoor`)))

(event `self.ReceiveTick`
  (params (DeltaSeconds :type "Float (single-precision)"))
  (bind _returnvalue (mod (.yaw (`Actor.K2_GetActorRotation` (`self.Actor`))) 360.0))
  (if (>= _returnvalue 58.0)
    (if (<= _returnvalue 62.0)
      (set `self.Complete` true)
      (else
        (set `self.Complete` false :!label _label)))
    (else
      (goto _label))))