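; OpeningDoor is a Blueprint for a puzzle door meant to open when stone tablets are rotated correctly.
; CheckingStonetabletRotation compares each tablet's rounded yaw to the matching RotationCheck entry, clearing the Check flag on any mismatch.
; The function never resets Check to true and prints a success message after the loop regardless of the result.
; No door movement is implemented, the event graph is empty, and nothing here calls the function.
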(fn `CheckingStonetabletRotation`
  (for (_array_element _array_index) (`self.StoneTablet`)
    (if (!= (`KismetMathLibrary.Round64` (.yaw (`self.K2_GetActorRotation` _array_element))) (`|GetArrayItem` (`self.RotationCheck`) _array_index))
      (set `self.Check` false)
      (elif (`self.Check`)
        (set `self.Check` true)
        (else
          (set `self.Check` false)))))
  (`KismetSystemLibrary.PrintString` "EveryThing is true we can open the door"))

(fn `UserConstructionScript`)