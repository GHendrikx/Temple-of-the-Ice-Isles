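; ChamberAudio is a trigger actor that plays a sequence of voice-over lines from Neva and Mimir when the ThirdPersonCharacter enters it.
; An IsPlaying flag lets the first overlap start the sequence only once, firing each audio event at the Box component's location.
; Three chained Timelines act as delays between lines, and the last one destroys the Box when it finishes.
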(event `self.ReceiveActorBeginOverlap`
  (params (OtherActor :type "Actor Object Reference"))
  (bind _returnvalue (`KismetMathLibrary.Conv_VectorToTransform` (`SceneComponent.K2_GetComponentLocation` (`self.Box`))))
  (cast `/Game/Blueprints/ThirdPersonBP/Blueprints/ThirdPersonCharacter` OtherActor)
  (if (not (`self.IsPlaying`))
    (set `self.IsPlaying` true)
    (`FMODBlueprintStatics.PlayEventAtLocation` "/Game/FMOD/Events/vo/neva/voice_lines/VO_Neva_03.VO_Neva_03" _returnvalue)
    (`Timeline|Timeline_0` :!via `PlayFromStart`
      (:`Finished`
        (`FMODBlueprintStatics.PlayEventAtLocation` "/Game/FMOD/Events/vo/mimir/VO_Mimir_05.VO_Mimir_05" _returnvalue)
        (`Timeline|Timeline_1` :!via `PlayFromStart`
          (:`Finished`
            (`FMODBlueprintStatics.PlayEventAtLocation` "/Game/FMOD/Events/vo/mimir/VO_Mimir_06.VO_Mimir_06" _returnvalue)
            (`Timeline|Timeline_2` :!via `PlayFromStart`
              (:`Finished`
                (`ActorComponent.K2_DestroyComponent` (`self.Box`))))))))))

(fn `UserConstructionScript`)