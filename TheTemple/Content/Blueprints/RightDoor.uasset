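; RightDoor is a door actor that swings its mesh open on Tick, with temple door audio.
; Each tick, while yaw plus a fixed step stays within OpenRotation, it fires the TempleDoor event, steps the yaw and plays a timeline.
; The timeline only serves as a delay before the Neva07 event plays.
; TestingDoor input handlers set and toggle EnableDoor, which controls only TempleDoor's AutoPlay, not the rotation.
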(event `InputAction|TestingDoor`
  (params (Key :type "Key Structure"))
  (:`Pressed`
    (set `self.EnableDoor` true)))

(event `self.ReceiveTick`
  (params (DeltaSeconds :type "Float (single-precision)"))
  (bind _staticmeshcomponent (`self.StaticMeshComponent`))
  (bind _returnvalue (`KismetMathLibrary.Conv_VectorToTransform` (`SceneComponent.K2_GetComponentLocation` (`self.StaticMeshComponent`))))
  (bind _returnvalue_2 (+ (.yaw (`SceneComponent.K2_GetComponentRotation` _staticmeshcomponent)) 5.0))
  (if (>= (`KismetMathLibrary.Conv_IntToDouble` (`self.OpenRotation`)) _returnvalue_2)
    (`FMODBlueprintStatics.PlayEventAtLocation` (`self.TempleDoor`) _returnvalue (`self.EnableDoor`))
    (`SceneComponent.K2_SetWorldRotation` _staticmeshcomponent (`KismetMathLibrary.MakeRotator` (.roll (`SceneComponent.K2_GetComponentRotation` _staticmeshcomponent)) (.pitch (`SceneComponent.K2_GetComponentRotation` _staticmeshcomponent)) _returnvalue_2) false false)
    (`Timeline|Timeline_0`
      (:`Finished`
        (`FMODBlueprintStatics.PlayEventAtLocation` (`self.Neva07`) _returnvalue)))))

(event `InputAction|TestingDoor`
  (params (Key :type "Key Structure"))
  (:`Pressed`
    (if (`self.EnableDoor`)
      (set `self.EnableDoor` false)
      (else
        (set `self.EnableDoor` true)))))

(fn `UserConstructionScript`)