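; A water actor that the player raises and lowers, and that respawns the third-person character on a hit.
; The WaterMechanic input axis moves the static mesh along Z, using AddingValue to check the new height against minimum and maximum levels.
; AddingValue has no explicit return for out-of-range heights, yet its output is always applied.
; A hit also shifts the world origin to a hard-coded BeginPosition set at BeginPlay.
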(event `self.ReceiveHit`
  (params (MyComp :type "PrimitiveComponent Object Reference") (Other :type "Actor Object Reference") (OtherComp :type "PrimitiveComponent Object Reference") (bSelfMoved :type Boolean) (HitLocation :type "Vector Structure") (HitNormal :type "Vector Structure") (NormalImpulse :type "Vector Structure") (Hit :type "HitResult Structure (by ref)"))
  (bind _asthird_person_character (cast `/Game/ThirdPersonBP/Blueprints/ThirdPersonCharacter` Other))
  (`/Game/ThirdPersonBP/Blueprints/ThirdPersonCharacter.Respawn` _asthird_person_character)
  (`GameplayStatics.SetWorldOriginLocation` (`KismetMathLibrary.FTruncVector` (`self.BeginPosition`))))

(event `self.ReceiveBeginPlay`
  (`self.EnableInput` (`GameplayStatics.GetPlayerController` 0))
  (set `self.BeginPosition` (-920.000366 -3560.0 -78.642029)))

(event `InputAction|SecondInteraction`
  (params (Key :type "Key Structure")))

(event `self.ReceiveTick`
  (params (DeltaSeconds :type "Float (single-precision)")))

(event `InputAxis|WaterMechanic`
  (params (AxisValue :type "Float (single-precision)"))
  (if (!= AxisValue 0.0)
    (bind _zaxus (`self.AddingValue` (.z (`SceneComponent.K2_GetComponentLocation` (`self.StaticMeshComponent`))) (* AxisValue 5.0)))
    (`SceneComponent.K2_SetWorldLocation` (`self.StaticMeshComponent`) (`KismetMathLibrary.MakeVector` (.x (`SceneComponent.K2_GetComponentLocation` (`self.StaticMeshComponent`))) (.y (`SceneComponent.K2_GetComponentLocation` (`self.StaticMeshComponent`))) _zaxus) false false)))

(fn `AddingValue`
  (params (ZAxis :type "Float (double-precision)") (FloatDirection :type "Float (double-precision)"))
  (returns (Zaxus :type "Float (double-precision)"))
  (set `self.Value` ZAxis)
  (bind _output_get (set `self.ReturnValue` (+ (`self.Value`) FloatDirection)))
  (bind _output_get_2 (set `self.FloatDirectionDownAllowed` (>= _output_get (`self.MinWaterLevel`))))
  (if _output_get_2
    (bind _output_get_3 (set `self.FloatDirectionUpAllowed` (<= _output_get (`self.MaxWaterLevel`))))
    (if _output_get_3
      (return (`self.ReturnValue`)))))

(fn `UserConstructionScript`)