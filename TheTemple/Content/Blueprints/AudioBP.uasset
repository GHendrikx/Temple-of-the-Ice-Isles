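; AudioBP is a one-shot trigger actor that plays a sequence of up to three audio message events when first overlapped.
; A HasPlayed flag blocks replays, and each event from the Messages array plays at the Box component's location.
; Timelines fed from the Timers array act as delays, each Finished output starting the next message after an array length check.
; The PlaySound graph is an empty stub.
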(event `self.ReceiveActorBeginOverlap`
  (params (OtherActor :type "Actor Object Reference"))
  (bind _timers (`self.Timers`))
  (bind _messages (`self.Messages`))
  (bind _returnvalue (`KismetArrayLibrary.Array_Length` (`self.Messages`)))
  (bind _returnvalue_2 (`KismetMathLibrary.Conv_VectorToTransform` (`SceneComponent.K2_GetComponentLocation` (`self.Box`))))
  (if (not (`self.HasPlayed`))
    (set `self.HasPlayed` true)
    (`FMODBlueprintStatics.PlayEventAtLocation` (`|GetArrayItem` _messages) _returnvalue_2)
    (`Timeline|Timeline_0` :`NewTime` (`|GetArrayItem` _timers) :!via `PlayFromStart`
      (:`Finished`
        (if (>= _returnvalue 1)
          (`FMODBlueprintStatics.PlayEventAtLocation` (`|GetArrayItem` _messages 1) _returnvalue_2)
          (`Timeline|Timeline_1` :`NewTime` (`|GetArrayItem` _timers 1)
            (:`Finished`
              (if (> _returnvalue 2)
                (`FMODBlueprintStatics.PlayEventAtLocation` (`|GetArrayItem` _messages 2) _returnvalue_2)
                (`Timeline|Timeline_2` :`NewTime` 12.0)))))))))

(fn `UserConstructionScript`)