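; Blueprint that watches the rotation of a stone tablet, apparently as an unfinished rotation check.
; Every Tick, it reads the world yaw of the StoneTablet's root component and tests it against a MinRotation to MaxRotation range.
; When the yaw is in range, it branches on the Rotate flag of IsRotating, but neither outcome triggers any action.
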(event `self.ReceiveTick`
  (params (DeltaSeconds :type "Float (single-precision)"))
  ;[1 1 1] Checking Rotation
  (if (`KismetMathLibrary.InRange_FloatFloat` (.yaw (`SceneComponent.K2_GetComponentRotation` (`Actor.RootComponent` (`self.StoneTablet`)))) (`self.MinRotation`) (`self.MaxRotation`))
    (if (`/Game/Blueprints/StoneTablet.Rotate` (`self.isRotating`))
      _)))