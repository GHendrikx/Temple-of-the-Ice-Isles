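; Visual Blueprint that shows or hides the actors of a visual layer according to a character's vision state.
; On BeginPlay it gathers the VisualLayer actors and hides each root component.
; ActivateVisual gathers the same actors and sets their root visibility to the passed Character's VisionActivated flag.
; Visibility changes do not propagate to child components, so only the roots are affected.
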(event `self.ReceiveBeginPlay`
  (bind _returnvalue (`LayersBlueprintLibrary.GetActors` (`self.visualLayer`)))
  (for _array_element _returnvalue
    (`SceneComponent.SetVisibility` (`Actor.RootComponent` _array_element) false false)))

(fn `ActivateVisual`
  (params (Character :type "/Game/ThirdPersonBP/Blueprints/ThirdPersonCharacter Object Reference"))
  (bind _returnvalue (`LayersBlueprintLibrary.GetActors` (`self.visualLayer`)))
  (for _array_element _returnvalue
    (`SceneComponent.SetVisibility` (`Actor.RootComponent` _array_element) (`/Game/ThirdPersonBP/Blueprints/ThirdPersonCharacter.VisionActivated` Character) false)))